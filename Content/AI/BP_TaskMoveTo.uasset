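; BP_TaskMoveTo is an AI task that walks an enemy along its route toward the core.
; On execute it copies the TargetPoints array from the controlled BP_EnemyMaster pawn.
; A self-calling event runs AIMoveTo to each point in order, advancing only on success, then moves the pawn to the BP_Core actor.
; The task never calls Finish Execute and does not handle failed moves.
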(event `self.ReceiveExecuteAI`
  (params (OwnerController :type "AIController Object Reference") (ControlledPawn :type "Pawn Object Reference"))
  ;[1 1 1] Hämta Target Points från Enemy
  (bind _asbp_enemy_master (cast `/Game/Enemies/BP_EnemyMaster` ControlledPawn))
  (set `self.TargetPoints` (`/Game/Enemies/BP_EnemyMaster.TargetPoints` _asbp_enemy_master))
  (`self.MoveThroughPoints`))

(event `MoveThroughPoints`
  (if (< (`self.currentTargetPointElement`) (`KismetArrayLibrary.Array_Length` (`self.TargetPoints`)))
    (`|AIMoveTo` (stale `self.ReceiveExecuteAI` ControlledPawn) (0.0 0.0 0.0) (`|GetArrayItem` (`self.TargetPoints`) (`self.currentTargetPointElement`)) 10.0
      (:`OnSuccess`
        (`/Engine/EditorBlueprintResources/StandardMacros.IncrementInt` (`self.currentTargetPointElement`)
          (:`  `
            (`self.MoveThroughPoints`)))))
    (else
      (bind _returnvalue (`GameplayStatics.GetActorOfClass` "/Game/CORE/BP_Core.BP_Core_C"))
      (`|AIMoveTo` (stale `self.ReceiveExecuteAI` ControlledPawn) (0.0 0.0 0.0) _returnvalue))))