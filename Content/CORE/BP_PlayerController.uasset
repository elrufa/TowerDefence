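; Player controller that handles the passive money income and build-mode cancelling.
; On BeginPlay it creates the money widget, adds it to the viewport and starts a looping timer that increments the money value stored on that widget.
; Right mouse click broadcasts the CancelBuildMode event dispatcher and clears the BuildModeActive flag.
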(event `self.ReceiveBeginPlay`
  ;[1 1 1] Skapa money widget sätt den aktiv, sätt timer som loopar var X-e sekund och kallar på AddMoney eventet
  (bind _returnvalue (`|CreateWidget` "/Game/UI/Widget_Money.Widget_Money_C"))
  (bind _output_get (set `self.MoneyWidget` _returnvalue))
  (`UserWidget.AddToViewport` (`self.MoneyWidget`) 0)
  (`KismetSystemLibrary.K2_SetTimerDelegate` (delegate `AddMoney`) 0.5 true))

(event `AddMoney`
  ;[1 1 1] Lägg till 1 money varje gång AddMoney kallas.
  (set `/Game/UI/Widget_Money.CurrentMoney` (+ (`/Game/UI/Widget_Money.CurrentMoney` (stale `self.ReceiveBeginPlay` _output_get)) 1) (stale `self.ReceiveBeginPlay` _output_get)))

(event `Key|RightMouseButton`
  (params (Key :type "Key Structure"))
  (:`Pressed`
    ;[1 1 1] Om högermusklick, skicka CancelBuildMode event dispatcher
    (`self.CancelBuildMode`)
    (set `self.BuildModeActive` false)))

(fn `UserConstructionScript`)