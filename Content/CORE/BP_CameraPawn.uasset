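; Camera pawn that gives the player a free-moving view, panned along world X and Y and zoomed by changing height.
; BeginPlay places it at a fixed starting location and pitch.
; Up/down and left/right axes shift it a fixed step per tick based only on input sign, so panning is frame-rate dependent.
; Zoom input offsets Z through FInterpTo scaled by delta time, with no height or bounds limits.
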(event `self.ReceiveBeginPlay`
  (`self.K2_SetActorLocationAndRotation` (-760.0 -60.0 1820.0) (`KismetMathLibrary.MakeRotator` 0.0 20.0)))

(event `InputAxis|InputZoom`
  (params (AxisValue :type "Float (single-precision)"))
  (bind (_returnvalue_x _returnvalue_y _returnvalue_z) (`KismetMathLibrary.BreakVector` (`self.K2_GetActorLocation`)))
  ;[1 1 1] Camera Controls
  (`self.K2_SetActorLocation` (`KismetMathLibrary.MakeVector` _returnvalue_x _returnvalue_y (`KismetMathLibrary.FInterpTo` _returnvalue_z (+ (* AxisValue -500.0) _returnvalue_z) (`GameplayStatics.GetWorldDeltaSeconds`) 10.0))))

(event `InputAxis|UpDownAxis`
  (params (AxisValue :type "Float (single-precision)"))
  (bind (_returnvalue_x _returnvalue_y _returnvalue_z) (`KismetMathLibrary.BreakVector` (`self.K2_GetActorLocation`)))
  (bind (_returnvalue_x_2 _returnvalue_y_2 _returnvalue_z_2) (`KismetMathLibrary.BreakVector` (`self.K2_GetActorLocation`)))
  ;[1 1 1] Camera Controls
  (if (< AxisValue 0.0)
    (`self.K2_SetActorLocation` (`KismetMathLibrary.MakeVector` (+ _returnvalue_x_2 -20.0) _returnvalue_y_2 _returnvalue_z_2))
    (elif (> AxisValue 0.0)
      (`self.K2_SetActorLocation` (`KismetMathLibrary.MakeVector` (+ _returnvalue_x 20.0) _returnvalue_y _returnvalue_z)))))

(event `InputAxis|LeftRightAxis`
  (params (AxisValue :type "Float (single-precision)"))
  (bind (_returnvalue_x _returnvalue_y _returnvalue_z) (`KismetMathLibrary.BreakVector` (`self.K2_GetActorLocation`)))
  (bind (_returnvalue_x_2 _returnvalue_y_2 _returnvalue_z_2) (`KismetMathLibrary.BreakVector` (`self.K2_GetActorLocation`)))
  ;[1 1 1] Camera Controls
  (if (< AxisValue 0.0)
    (`self.K2_SetActorLocation` (`KismetMathLibrary.MakeVector` _returnvalue_x (+ _returnvalue_y -20.0) _returnvalue_z))
    (elif (> AxisValue 0.0)
      (`self.K2_SetActorLocation` (`KismetMathLibrary.MakeVector` _returnvalue_x_2 (+ _returnvalue_y_2 20.0) _returnvalue_z_2)))))

(fn `UserConstructionScript`)