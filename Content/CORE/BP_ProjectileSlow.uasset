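; A tower projectile that homes on its target enemy, deals damage and applies a slow.
; Tick moves it toward TargetEnemy at constant speed, destroying it if the target is invalid.
; Overlapping any BP_EnemyMaster subtracts damage from the "Standard" tower data row, applies Slowed, destroys the projectile and runs the death check.
; Tick reads ProjectileSpeed from that same row lookup, which only executes on overlap.
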(event `self.ReceiveActorBeginOverlap`
  (params (OtherActor :type "Actor Object Reference"))
  ;[1 1 1] Damage Target Enemy
  (bind _returnvalue (`|GetDataTableRow` "/Game/Towers/TowerDataTable.TowerDataTable" "Standard")
    (:`then`
      (bind _asbp_enemy_master (cast `/Game/Enemies/BP_EnemyMaster` OtherActor))
      (set `/Game/Enemies/BP_EnemyMaster.Health` (- (`/Game/Enemies/BP_EnemyMaster.Health` _asbp_enemy_master) (`.Damage_2_65EEE6FD4A822C31FD4A0EAD83BEAA08` (break `/Game/Towers/TowerStruct` _returnvalue))) _asbp_enemy_master)
      (`/Game/Enemies/BP_EnemyMaster.Slowed` _asbp_enemy_master (`self.SlowDuration`) (`self.SlowPercent`))
      (`self.K2_DestroyActor`)
      (`/Game/Enemies/BP_EnemyMaster.CheckIsDead` _asbp_enemy_master))))

(event `self.ReceiveTick`
  (params (DeltaSeconds :type "Float (single-precision)"))
  (bind _targetenemy (`self.TargetEnemy`))
  (`/Engine/EditorBlueprintResources/StandardMacros.IsValid` _targetenemy
    (:`Is Valid`
      (`self.K2_SetActorLocation` (`KismetMathLibrary.VInterpTo_Constant` (`self.K2_GetActorLocation`) (`self.K2_GetActorLocation` _targetenemy) DeltaSeconds (`.ProjectileSpeed_9_7B5523D24D95300DA754CB895A37F5DA` (break `/Game/Towers/TowerStruct` (stale `self.ReceiveActorBeginOverlap` _returnvalue))))))
    (:`Is Not Valid`
      (`self.K2_DestroyActor`))))

(fn `UserConstructionScript`)