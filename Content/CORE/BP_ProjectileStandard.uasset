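; Standard tower projectile that flies to the position its TargetEnemy held at BeginPlay, without homing.
; Overlapping any BP_EnemyMaster subtracts the TowerDataTable "Standard" row's Damage from Health, calls CheckIsDead and destroys the projectile.
; Tick moves it with VInterpToConstant and destroys it after a two-second delay.
; Its ProjectileSpeed comes from the row lookup that runs only on overlap, so it is unset during flight.
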(event `self.ReceiveBeginPlay`
  (set `self.LastKnownLocation` (`self.K2_GetActorLocation` (`self.TargetEnemy`))))

(event `self.ReceiveActorBeginOverlap`
  (params (OtherActor :type "Actor Object Reference"))
  ;[1 1 1] Damage Target Enemy
  (bind _returnvalue (`|GetDataTableRow` "/Game/Towers/TowerDataTable.TowerDataTable" "Standard")
    (:`then`
      (bind _asbp_enemy_master (cast `/Game/Enemies/BP_EnemyMaster` OtherActor))
      (set `/Game/Enemies/BP_EnemyMaster.Health` (- (`/Game/Enemies/BP_EnemyMaster.Health` _asbp_enemy_master) (break `/Game/Towers/TowerStruct` _returnvalue)) _asbp_enemy_master)
      (`/Game/Enemies/BP_EnemyMaster.CheckIsDead` _asbp_enemy_master)
      (`self.K2_DestroyActor`))))

(event `self.ReceiveTick`
  (params (DeltaSeconds :type "Float (single-precision)"))
  (`self.K2_SetActorLocation` (`KismetMathLibrary.VInterpTo_Constant` (`self.K2_GetActorLocation`) (`self.LastKnownLocation`) DeltaSeconds (`.ProjectileSpeed_9_7B5523D24D95300DA754CB895A37F5DA` (break `/Game/Towers/TowerStruct` (stale `self.ReceiveActorBeginOverlap` _returnvalue)))))
  (`KismetSystemLibrary.Delay` 2.0)
  (`self.K2_DestroyActor`))

(fn `UserConstructionScript`)