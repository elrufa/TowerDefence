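; BP_Core is the base that enemies attack, tracking its health through an on-screen Widget_Core.
; On BeginPlay it creates that widget and adds it to the viewport.
; When a BP_EnemyMaster overlaps it, the enemy's Strength is subtracted from CoreHealth stored in the widget, the health bar updates, and the enemy is destroyed.
; At zero health or below it calls the widget's IsDead.
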(event `self.ReceiveBeginPlay`
  (bind _returnvalue (`|CreateWidget` "/Game/UI/Widget_Core.Widget_Core_C"))
  (bind _output_get (set `self.WidgetCoreReference` _returnvalue))
  (`UserWidget.AddToViewport` _output_get 0))

(event `self.ReceiveActorBeginOverlap`
  (params (OtherActor :type "Actor Object Reference"))
  (bind _widgetcorereference (`self.WidgetCoreReference`))
  (bind _corehealth (`/Game/UI/Widget_Core.CoreHealth` _widgetcorereference))
  (bind _asbp_enemy_master (cast `/Game/Enemies/BP_EnemyMaster` OtherActor))
  (bind _output_get (set `/Game/UI/Widget_Core.CoreHealth` (- _corehealth (`/Game/Enemies/BP_EnemyMaster.Strength` _asbp_enemy_master)) _widgetcorereference))
  (`ProgressBar.SetPercent` (`/Game/UI/Widget_Core.CoreHealthBar` _widgetcorereference) (* _output_get 0.01))
  (`self.K2_DestroyActor` _asbp_enemy_master)
  (if (<= _corehealth 0.0)
    (`/Game/UI/Widget_Core.IsDead` (`self.WidgetCoreReference`))))

(fn `UserConstructionScript`)