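; Wave spawner that runs a countdown UI and spawns standard enemies during waves.
; A looping timer updates the Widget_Waves countdown, pauses at zero and triggers the next wave, with Wave2 still empty.
; Wave1 repeatedly spawns AI enemies at the spawner while the countdown is zero; an input action spawns one near world origin.
; After a delay the countdown resets and, unless on wave five, resumes, updates completion text and destroys the spawner.
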(event `SpawnEnemy`
  (bind (_returnvalue_x _returnvalue_y) (`KismetMathLibrary.BreakVector` (`KismetMathLibrary.RandomUnitVector`)))
  (`|SpawnActorFromClass` "/Game/Enemies/BP_EnemyStandard.BP_EnemyStandard_C" (`KismetMathLibrary.MakeTransform` (`KismetMathLibrary.MakeVector` (* _returnvalue_x 200.0) (* _returnvalue_y 200.0))) "Undefined" "OverrideRootScale" null null))

(event `InputAction|SpawnEnemy`
  (params (Key :type "Key Structure"))
  (:`Pressed`
    (`self.SpawnEnemy`)))

(event `self.ReceiveBeginPlay`
  ;[1 1 1] Create and add Wave UI to viewport.
  (bind _returnvalue (`|CreateWidget` "/Game/UI/Widget_Waves.Widget_Waves_C"))
  (bind _output_get (set `self.WidgetWaveReference` _returnvalue))
  (`UserWidget.AddToViewport` _output_get 0)
  (`KismetSystemLibrary.K2_SetTimerDelegate` (delegate `CountUntilNextWave`) 1.0 true))

(event `CountUntilNextWave`
  (bind _widgetwavereference (`self.WidgetWaveReference`))
  (bind _output_get (set `self.UntilNextWave` (- (`self.UntilNextWave`) 1)))
  (`TextBlock.SetText` (`/Game/UI/Widget_Waves.CountDownUntilNextWaveText` (stale `self.ReceiveBeginPlay` _output_get)) (`KismetTextLibrary.Conv_IntToText` _output_get))
  (if (== (`self.UntilNextWave`) 0)
    (`KismetSystemLibrary.K2_PauseTimer` null "CountUntilNextWave")
    (`TextBlock.SetColorAndOpacity` (`/Game/UI/Widget_Waves.CountDownUntilNextWaveText` (`self.WidgetWaveReference`)) (make `SlateColor` (struct :`R` 1.0 :`A` 1.0)))
    (bind _output_get_2 (set `self.WhichWaveToTrigger` (+ (`self.WhichWaveToTrigger`) 1)))
    (`TextBlock.SetText` (`/Game/UI/Widget_Waves.WaveNumberText` (`self.WidgetWaveReference`)) (`KismetTextLibrary.Conv_IntToText` _output_get_2))
    (`|ExecutionSequence`
      (:`then_0`
        (if (== (`self.WhichWaveToTrigger`) 1)
          (`self.Wave1`)
          (`KismetSystemLibrary.Delay` 30.0 :!label _label)
          (set `self.UntilNextWave` 30)
          (`TextBlock.SetColorAndOpacity` (`/Game/UI/Widget_Waves.CountDownUntilNextWaveText` (`self.WidgetWaveReference`)) (make `SlateColor` (struct :`G` 1.0 :`B` 0.007175 :`A` 1.0)))
          (if (not (== (`self.WhichWaveToTrigger`) 5))
            (`KismetSystemLibrary.K2_UnPauseTimer` null "CountUntilNextWave")
            (`TextBlock.SetOpacity` (`/Game/UI/Widget_Waves.WaveCompletedText` _widgetwavereference) 1.0)
            (`TextBlock.SetOpacity` (`/Game/UI/Widget_Waves.WaveNumberText` _widgetwavereference) 0.0)
            (`TextBlock.SetOpacity` (`/Game/UI/Widget_Waves.WaveCompletedText` _widgetwavereference) 0.0)
            (`self.K2_DestroyActor`))))
      (:`then_1`
        (if (== (`self.WhichWaveToTrigger`) 2)
          (`self.Wave2`)
          (goto _label))))))

(event `Wave1`
  (`KismetSystemLibrary.K2_SetTimerDelegate` (delegate `SpawnStandardEnemy1`) 3.0 true))

(event `SpawnStandardEnemy1`
  (if (== (`self.UntilNextWave`) 0)
    (`AIBlueprintHelperLibrary.SpawnAIFromClass` "/Game/Enemies/BP_EnemyStandard.BP_EnemyStandard_C" "/Game/AI/AI_BehaviourTree.AI_BehaviourTree" (`self.K2_GetActorLocation`) (struct) false null)))

(event `Wave2`)

(fn `UserConstructionScript`)