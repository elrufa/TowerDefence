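; BP_EnemyMaster is an enemy character Blueprint, named as the master enemy, that handles damage, death and slow effects.
; TakeDamage prints the amount, subtracts it from Health and calls CheckIsDead, which destroys the actor at zero or below.
; Slowed scales max walk speed and swaps the Cone material, then restores the saved speed and red material after a delay.
; An IsSlowed flag ignores repeated slows while one is active.
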(event `self.ReceiveTick`
  (params (DeltaSeconds :type "Float (single-precision)")))

(event `CheckIsDead`
  (if (<= (`self.Health`) 0.0)
    (`self.K2_DestroyActor`)))

(event `Slowed`
  (params (slowedDuration :type "Float (double-precision)") (percentSlow :type "Float (double-precision)"))
  (bind _charactermovement (`self.CharacterMovement`))
  (if (not (`self.isSlowed`))
    ;[1 1 1] Sätt fiende som "slowed". Spara orginal-speed i temp variable. Modifiera max walk speed med percent slow från input
    (set `self.isSlowed` true)
    (bind _output_get (set `self.standardSpeed` (`CharacterMovementComponent.MaxWalkSpeed` _charactermovement)))
    (set `CharacterMovementComponent.MaxWalkSpeed` (* _output_get percentSlow) _charactermovement)
    (`PrimitiveComponent.SetMaterial` (`self.Cone`) 0 "/Game/Material/MI_Slowed.MI_Slowed")
    ;[1 1 1] Vänta i x sekunder (från input slowduration). Återställ därefter speed till standard med hjälp av tempvariabeln.
    (`KismetSystemLibrary.Delay` slowedDuration)
    (set `CharacterMovementComponent.MaxWalkSpeed` (`self.standardSpeed`) _charactermovement)
    (set `self.isSlowed` false)
    (`PrimitiveComponent.SetMaterial` (`self.Cone`) 0 "/Game/Material/MI_Red.MI_Red")))

(event `TakeDamage`
  (params (Damage :type "Float (double-precision)"))
  (`KismetSystemLibrary.PrintString` (`KismetStringLibrary.Concat_StrStr` "Enemy Took " (`KismetStringLibrary.Conv_DoubleToString` Damage) "damage!"))
  (set `self.Health` (- (`self.Health`) Damage))
  (`self.CheckIsDead`))

(fn `UserConstructionScript`)