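; BP_TurretProjectile is a homing turret projectile that damages a single target enemy.
; Each tick it moves toward the enemy's current location at constant speed, using VInterpToConstant and an unswept SetActorLocation with no validity check on the target.
; When its sphere collider overlaps that target, it subtracts a fixed amount of Health, calls the enemy's CheckIsDead and destroys itself, ignoring other actors.
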(event `self.ReceiveTick`
  (params (DeltaSeconds :type "Float (single-precision)"))
  (`self.K2_SetActorLocation` (`KismetMathLibrary.VInterpTo_Constant` (`self.K2_GetActorLocation`) (`self.K2_GetActorLocation` (`self.TargetEnemy`)) DeltaSeconds (`self.Projectile Speed`))))

(event `self.SphereCol.OnComponentBeginOverlap`
  (params (OverlappedComponent :type "PrimitiveComponent Object Reference") (OtherActor :type "Actor Object Reference") (OtherComp :type "PrimitiveComponent Object Reference") (OtherBodyIndex :type Integer) (bFromSweep :type Boolean) (SweepResult :type "HitResult Structure (by ref)"))
  (bind _targetenemy (`self.TargetEnemy`))
  (if (== OtherActor _targetenemy)
    (set `/Game/Enemies/BP_EnemyMaster.Health` (- (`/Game/Enemies/BP_EnemyMaster.Health` _targetenemy) 10.0) _targetenemy)
    (`/Game/Enemies/BP_EnemyMaster.CheckIsDead` _targetenemy)
    (`self.K2_DestroyActor`)))

(fn `UserConstructionScript`)