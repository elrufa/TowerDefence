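; Standard tower-defense turret that periodically fires at the enemy closest to reaching the core.
; On BeginPlay it reads the "Standard" data table row to size its range sphere and start a looping fire timer.
; Each shot picks the overlapping enemy with the lowest navigation path cost to BP_Core and spawns a projectile targeting it.
; A nearest-to-tower targeting function also exists but is not called here.
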(event `self.ReceiveBeginPlay`
  (bind _returnvalue (`|GetDataTableRow` "/Game/Towers/TowerDataTable.TowerDataTable" "Standard")
    (:`then`
      (`SphereComponent.SetSphereRadius` (`self.Sphere`) (break `/Game/Towers/TowerStruct` _returnvalue) true)
      (`KismetSystemLibrary.K2_SetTimerDelegate` (delegate `Fire`) (`.FireRate_8_416E7B744646D7F50A542CAE3565F67C` (break `/Game/Towers/TowerStruct` _returnvalue)) true))))

(event `Fire`
  (bind _targetenemy (`self.Get Enemy Closest to Goal` (`self.GetOverlappingActors` "/Game/Enemies/BP_EnemyMaster.BP_EnemyMaster_C")))
  (bind _asbp_enemy_master (cast `/Game/Enemies/BP_EnemyMaster` _targetenemy))
  (`/Engine/EditorBlueprintResources/StandardMacros.IsValid` _asbp_enemy_master
    (:`Is Valid`
      (`|SpawnActorFromClass` "/Game/CORE/BP_ProjectileStandard.BP_ProjectileStandard_C" (`self.GetTransform`) "Undefined" "OverrideRootScale" null _asbp_enemy_master null))))

(fn `Get Closest Target`
  (params (ListOfEnemies :type "Array of Actor Object Reference"))
  (returns (ClosestTarget :type "Actor Object Reference"))
  (for _array_element ListOfEnemies
    (`self.TempTarget`
      (:`then`
        (bind _returnvalue (`self.GetDistanceTo` _array_element))
        (if (< _returnvalue (`self.TempDistance`))
          (set `self.TempTarget` _array_element)
          (set `self.TempDistance` _returnvalue)))
      (:`else`
        (set `self.TempTarget` _array_element)
        (set `self.TempDistance` (`self.GetDistanceTo` _array_element)))))
  (return (`self.TempTarget`)))

(fn `Get Enemy Closest to Goal`
  (params (ListOfEnemies :type "Array of Actor Object Reference"))
  (returns (TargetEnemy :type "Actor Object Reference"))
  (locals (TargetCurrentlyChecking :type "Actor Object Reference") (CurrentClosestDistance :type "Float (double-precision)"))
  (for _array_element ListOfEnemies
    (`local.TargetCurrentlyChecking`
      (:`then`
        ;[1 1 1] Checka Path Cost för current looping element mot CurrentClosestDistance. Om det är mindre (närmre målet), byt target och sätt ny current closest distance.
        (bind _returnvalue (`GameplayStatics.GetActorOfClass` "/Game/CORE/BP_Core.BP_Core_C"))
        (bind _pathcost (`NavigationSystemV1.GetPathCost` (`self.K2_GetActorLocation` _array_element) (`self.K2_GetActorLocation` _returnvalue) null null))
        (if (< _pathcost (`local.CurrentClosestDistance`))
          (set `local.TargetCurrentlyChecking` _array_element)
          (set `local.CurrentClosestDistance` _pathcost)))
      (:`else`
        ;[1 1 1] Händer första gången/om TargetCurrentlyChecking inte har ett värde.
        ; Sätt target till current looping target. Kolla avstånd kvar till Core och sätt CurrentClosestDistance till resultatet.
        (bind _output_get (set `local.TargetCurrentlyChecking` _array_element))
        (bind _returnvalue_2 (`GameplayStatics.GetActorOfClass` "/Game/CORE/BP_Core.BP_Core_C"))
        (set `local.CurrentClosestDistance` (`NavigationSystemV1.GetPathCost` (`self.K2_GetActorLocation` _output_get) (`self.K2_GetActorLocation` _returnvalue_2) null null)))))
  (return (`local.TargetCurrentlyChecking`)))

(fn `UserConstructionScript`)