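; Base tower for a tower defense game that automatically shoots the in-range enemy nearest the goal.
; The construction script uses the tower type's data table row to set stats, range sphere radius and mesh.
; A looping fire-rate timer ranks overlapping enemies by navigation path cost to BP_Core rather than straight-line distance.
; It spawns the configured projectile at the tower, passing it the target, damage and speed.
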(event `self.ReceiveBeginPlay`
  (bind (_towerstats_rangeradius _towerstats_firerate _towerstats_damage _towerstats_projectiletype _towerstats_cost _towerstats_projectilespeed) (break `/Game/Towers/TowerStruct` (`self.TowerStats`)))
  ;[1 1 1] Start looping EnemyShoot-finder and shoot target in range that is closest to goal
  (`KismetSystemLibrary.K2_SetTimerDelegate` (delegate `SearchAndDestroy`) _towerstats_firerate true))

(event `SearchAndDestroy`
  (bind (_towerstats_rangeradius _towerstats_firerate _towerstats_damage _towerstats_projectiletype _towerstats_cost _towerstats_projectilespeed) (break `/Game/Towers/TowerStruct` (`self.TowerStats`)))
  ;[1 1 1] Start looping EnemyShoot-finder and shoot target in range that is closest to goal
  (bind _enemyclosesttogoal (`self.Find Enemy Closest To Goal` (`PrimitiveComponent.GetOverlappingActors` (`self.TowerRangeSphere`) "/Game/Enemies/BP_EnemyMaster.BP_EnemyMaster_C")))
  (`/Engine/EditorBlueprintResources/StandardMacros.IsValid` _enemyclosesttogoal
    (:`Is Valid`
      (bind _asbp_enemy_master (cast `/Game/Enemies/BP_EnemyMaster` _enemyclosesttogoal))
      (`|SpawnActorFromClass` _towerstats_projectiletype (`KismetMathLibrary.Conv_VectorToTransform` (`self.K2_GetActorLocation`)) "AlwaysSpawn" "OverrideRootScale" null _asbp_enemy_master _towerstats_damage _towerstats_projectilespeed null))))

(fn `Find Enemy Closest To Goal`
  (params (ListOfEnemies :type "Array of Actor Object Reference"))
  (returns (EnemyClosestToGoal :type "Actor Object Reference"))
  (locals (CurrentClosestTarget :type "Actor Object Reference") (CurrentClosestDiance :type "Float (double-precision)"))
  (bind _currentclosesttarget (`local.CurrentClosestTarget`))
  (for _array_element ListOfEnemies
    (`local.CurrentClosestTarget`
      (:`then`
        ;[1 1 1] Checka Path Cost för current looping element mot CurrentClosestDistance. Om det är mindre (närmre målet), byt target och sätt ny current closest distance.
        (bind _returnvalue (`GameplayStatics.GetActorOfClass` "/Game/CORE/BP_Core.BP_Core_C"))
        (bind _pathcost (`NavigationSystemV1.GetPathCost` (`self.K2_GetActorLocation` _array_element) (`self.K2_GetActorLocation` _returnvalue) null null))
        (if (< _pathcost (`local.CurrentClosestDiance`))
          (set `local.CurrentClosestTarget` _array_element)
          (set `local.CurrentClosestDiance` _pathcost)))
      (:`else`
        ;[1 1 1] Händer första gången/om TargetCurrentlyChecking inte har ett värde.
        ; Sätt target till current looping target. Kolla avstånd kvar till Core och sätt CurrentClosestDistance till resultatet.
        (bind _output_get (set `local.CurrentClosestTarget` _array_element))
        (bind _returnvalue_2 (`GameplayStatics.GetActorOfClass` "/Game/CORE/BP_Core.BP_Core_C"))
        (set `local.CurrentClosestDiance` (`NavigationSystemV1.GetPathCost` (`self.K2_GetActorLocation` _output_get) (`self.K2_GetActorLocation` _returnvalue_2) null null)))))
  (`KismetSystemLibrary.PrintString` (`KismetSystemLibrary.GetDisplayName` _currentclosesttarget))
  (return _currentclosesttarget))

(fn `UserConstructionScript`
  (bind _returnvalue (`|GetDataTableRow` "/Game/Towers/TowerDataTable.TowerDataTable" (`self.TypeOfTower`))
    (:`then`
      (bind _output_get (set `self.TowerStats` _returnvalue))
      (`SphereComponent.SetSphereRadius` (`self.TowerRangeSphere`) (break `/Game/Towers/TowerStruct` _output_get) true)
      (`StaticMeshComponent.SetStaticMesh` (`self.StaticMesh`) (`.TowerMesh_18_F6529AAF44A8DB2865641AB8FA733FF4` (break `/Game/Towers/TowerStruct` _output_get))))))