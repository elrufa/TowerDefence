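; BP_ProjectileMaster is a homing tower projectile, apparently a base class, that chases a Target actor and damages it on contact.
; Each Tick it moves toward the Target's current location at constant ProjectileSpeed via VInterpToConstant without sweeping, or destroys itself if the Target is invalid.
; Overlapping the Target prints a debug message, calls TakeDamage with Damage and destroys the projectile, while other overlapping actors are ignored.
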(event `self.ReceiveActorBeginOverlap`
  (params (OtherActor :type "Actor Object Reference"))
  (if (== OtherActor (`self.Target`))
    (`KismetSystemLibrary.PrintString` "Hit Target. DAMAGE!")
    (`/Game/Enemies/BP_EnemyMaster.TakeDamage` (`self.Target`) (`self.Damage`))
    (`self.K2_DestroyActor`)))

(event `self.ReceiveTick`
  (params (DeltaSeconds :type "Float (single-precision)"))
  (`/Engine/EditorBlueprintResources/StandardMacros.IsValid` (`self.Target`)
    (:`Is Valid`
      (`self.K2_SetActorLocation` (`KismetMathLibrary.VInterpTo_Constant` (`self.K2_GetActorLocation`) (`self.K2_GetActorLocation` (`self.Target`)) (`GameplayStatics.GetWorldDeltaSeconds`) (`self.ProjectileSpeed`))))
    (:`Is Not Valid`
      (`self.K2_DestroyActor`))))

(fn `UserConstructionScript`)