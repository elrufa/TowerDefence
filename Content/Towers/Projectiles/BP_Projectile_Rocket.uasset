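; Rocket tower projectile that deals splash damage to enemies when it overlaps its assigned Target.
; On that overlap, a sphere query centered on the target gathers BP_EnemyMaster pawns within SplashRadius and applies the full Damage to each, with no falloff.
; A debug sphere and a printed hit count show each blast.
; This graph contains no movement or self-destroy logic.
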(event `self.ReceiveActorBeginOverlap`
  (params (OtherActor :type "Actor Object Reference"))
  (bind _returnvalue (`self.K2_GetActorLocation` OtherActor))
  (if (== OtherActor (`self.Target`))
    (`KismetSystemLibrary.DrawDebugSphere` _returnvalue (`self.SplashRadius`) 24 (struct :`R` 1.0 :`A` 1.0) 2.0 2.0)
    (bind _outactors (`KismetSystemLibrary.SphereOverlapActors` _returnvalue (`self.SplashRadius`) (`|MakeArray` "ObjectTypeQuery3" :!type "EObjectTypeQuery Enum") "/Game/Enemies/BP_EnemyMaster.BP_EnemyMaster_C"))
    (`KismetSystemLibrary.PrintString` (`KismetStringLibrary.Conv_IntToString` (`KismetArrayLibrary.Array_Length` _outactors)))
    (for _array_element _outactors
      (bind _asbp_enemy_master (cast `/Game/Enemies/BP_EnemyMaster` _array_element))
      (`/Game/Enemies/BP_EnemyMaster.TakeDamage` _asbp_enemy_master (`self.Damage`)))))

(fn `UserConstructionScript`)