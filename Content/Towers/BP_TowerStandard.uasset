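; Standard tower that automatically shoots at the nearest enemy within its range.
; On BeginPlay it reads the "Standard" data table row to size its range sphere and start a looping fire timer.
; Each tick of that timer picks the closest overlapping BP_EnemyMaster through a linear distance search and spawns a BP_ProjectileStandard at the tower's transform, passing that enemy as its target.
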(event `self.ReceiveBeginPlay`
  (bind _returnvalue (`|GetDataTableRow` "/Game/Towers/TowerDataTable.TowerDataTable" "Standard")
    (:`then`
      (`SphereComponent.SetSphereRadius` (`self.Sphere`) (`.Range_7_ED5FCDDE42D380AEDF38098DC1C565CF` (break `/Game/Towers/TowerStruct` _returnvalue)) true)
      (`KismetSystemLibrary.K2_SetTimerDelegate` (delegate `Fire`) (`.FireRate_8_416E7B744646D7F50A542CAE3565F67C` (break `/Game/Towers/TowerStruct` _returnvalue)) true))))

(event `Fire`
  (bind _closesttarget (`self.Get Closest Target` (`self.GetOverlappingActors` "/Game/Enemies/BP_EnemyMaster.BP_EnemyMaster_C")))
  (bind _asbp_enemy_master (cast `/Game/Enemies/BP_EnemyMaster` _closesttarget))
  (`/Engine/EditorBlueprintResources/StandardMacros.IsValid` _asbp_enemy_master
    (:`Is Valid`
      (`|SpawnActorFromClass` "/Game/CORE/BP_ProjectileStandard.BP_ProjectileStandard_C" (`self.GetTransform`) "Undefined" "OverrideRootScale" null _asbp_enemy_master null))))

(fn `Get Closest Target`
  (params (ListOfEnemies :type "Array of Actor Object Reference"))
  (returns (ClosestTarget :type "Actor Object Reference"))
  (for _array_element ListOfEnemies
    (`self.TempTarget`
      (:`then`
        (bind _returnvalue (`self.GetDistanceTo` _array_element))
        (if (< _returnvalue (`self.TempDistance`))
          (set `self.TempTarget` _array_element)
          (set `self.TempDistance` _returnvalue)))
      (:`else`
        (set `self.TempTarget` _array_element)
        (set `self.TempDistance` (`self.GetDistanceTo` _array_element)))))
  (return (`self.TempTarget`)))

(fn `UserConstructionScript`)